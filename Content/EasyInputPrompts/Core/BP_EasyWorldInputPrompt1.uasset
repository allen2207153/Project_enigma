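; World-placed input prompt actor that shows key icons and text for mapped actions or keys while something overlaps its sphere.
; On BeginPlay it creates a multi-input prompt widget, assigns it to its widget component and hides it; sphere overlaps toggle visibility.
; Key image size and text styling come from CalculateFinalResolution, and component scale is divided by ResolutionMultiplier.
; The construction script applies DisplayType as the widget space.
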(event OnComponentBeginOverlap(Sphere)
  (params (OverlappedComponent :type Primitive%20Component%20Object%20Reference) (OtherActor :type Actor%20Object%20Reference) (OtherComp :type Primitive%20Component%20Object%20Reference) (OtherBodyIndex :type Integer) (bFromSweep :type Boolean) (SweepResult :type Hit%20Result%20Structure%20%28by%20ref%29))
  (Rendering|SetVisibility (Variables|Default|GetWidget) true false))

(event OnComponentEndOverlap(Sphere)
  (params (OverlappedComponent :type Primitive%20Component%20Object%20Reference) (OtherActor :type Actor%20Object%20Reference) (OtherComp :type Primitive%20Component%20Object%20Reference) (OtherBodyIndex :type Integer))
  (Rendering|SetVisibility (Variables|Default|GetWidget) false false))

(event EventBeginPlay
  (bind (_returnvalue _textstyling) (|CalculateFinalResolution))
  (bind _returnvalue_2 (UserInterface|CreateWidget "/Game/EasyInputPrompts/Core/WBP_EasyMultiInputPromptDisplayer.WBP_EasyMultiInputPromptDisplayer_C" 0 (Variables|EasyConfig|Keys|GetUse%20Input%20Action?) (Variables|EasyConfig|Keys|GetInput%20Action) (Variables|EasyConfig|Keys|GetInput%20Mapping%20Context) (Variables|EasyConfig|Keys|GetMNK%20Keys) (Variables|EasyConfig|Keys|GetGamepad%20Keys) _returnvalue (Variables|EasyConfig|Styling|GetText%20To%20Display) _textstyling (Variables|EasyConfig|Styling|GetText%20Color) (Variables|EasyConfig|Styling|GetText%20Position) (Variables|EasyConfig|Styling|GetText%20Padding) (Variables|EasyConfig|Styling|GetIcon%20Color) (Variables|EasyConfig|Styling|GetSpacing) (Variables|EasyConfig|Keys|GetHide%20Key%20For%20Other%20Devices?) (Variables|EasyConfig|Keys|GetHideTextAsWell?)))
  (bind _output_get (Variables|Components|SetMutliInputPromptWidgetReference _returnvalue_2))
  (UserInterface|SetWidget (Variables|Default|GetWidget) _output_get)
  (|UpdateWidgetScale)
  (Rendering|SetVisibility (Variables|Default|GetWidget) false false))

(fn ConstructionScript
  (Class|WidgetComponent|SetWidgetSpace (Variables|Default|GetWidget) (Variables|EasyConfig|Styling|GetDisplayType)))